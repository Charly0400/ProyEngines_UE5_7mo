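; Base enemy NPC with health, a looping zombie melee attack animation and ragdoll death.
; MeleeTrace hits apply damage to the struck actor, while incoming damage lowers clamped Health.
; At zero Health it increments the game mode's kill counter, ragdolls the mesh, disables movement and unpossesses.
; A looping timer then destroys the body once the player is not on top of it; IsDead? is a stub returning false.
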(event OnTraceHit(MeleeTrace)
  (params (ThisComponent :type Melee%20Trace%20Component%20Object%20Reference) (HitActor :type Actor%20Object%20Reference) (HitLocation :type Vector%20%28by%20ref%29 :default "0, 0, 0") (HitNormal :type Vector%20%28by%20ref%29 :default "0, 0, 0") (HitBoneName :type Name :default "None"))
  (Game|Damage|ApplyDamage HitActor (Variables|Default|GetDamage) 0 0))

(event Custom|DestroyActorEvent
  ;[0.02 0.02 0.02] Take Damage from Player and Update HUD counter
  (if (> (Math|Vector|Distance(Vector) (Transformation|GetActorLocation (Game|GetPlayerCharacter 0)) (Transformation|GetActorLocation)) 5.0)
    (Actor|DestroyActor)))

(event EventMeleeAttack
  (Components|Animation|PlayAnimation (Variables|Character|GetMesh) "/Game/Characters/Zombie/Animations/Zombie_Attack.Zombie_Attack" true))

(event Collision|EventHit
  (params (MyComp :type Primitive%20Component%20Object%20Reference) (Other :type Actor%20Object%20Reference) (OtherComp :type Primitive%20Component%20Object%20Reference) (bSelfMoved :type Boolean) (HitLocation :type Vector :default "0, 0, 0") (HitNormal :type Vector :default "0, 0, 0") (NormalImpulse :type Vector :default "0, 0, 0") (Hit :type Hit%20Result%20Structure%20%28by%20ref%29)))

(event Game|Damage|EventAnyDamage
  (params (Damage :type Float%20%28single-precision%29) (DamageType :type Damage%20Type%20Object%20Reference) (InstigatedBy :type Controller%20Object%20Reference) (DamageCauser :type Actor%20Object%20Reference))
  ;[0.02 0.02 0.02] Take Damage from Player and Update HUD counter
  (bind _output_get (Variables|Default|SetHealth (Math|Float|Clamp(Float) (- (Variables|Default|GetHealth) Damage) 0.0 1e+02)))
  (if (<= _output_get 0.0)
    (bind _asbp_third_person_game_mode (Utilities|Casting|CastToBP_ThirdPersonGameMode (Game|GetGameMode)))
    (Math|Integer|IncrementInt (Variables|/Game/ThirdPerson/Blueprints/BP_ThirdPersonGameMode.BP_ThirdPersonGameMode_C|GetEnemysDestroy _asbp_third_person_game_mode)
      (:%20%20
        (CallFunction|Died)
        (Utilities|Time|SetTimerbyEvent (delegate Custom|DestroyActorEvent) 1e+01 true)))))

(fn ConstructionScript)

(fn Died
  (Physics|SetSimulatePhysics (Variables|Character|GetMesh) true)
  (Collision|SetCollisionEnabled (Variables|Character|GetMesh) "PhysicsOnly")
  (Collision|SetCollisionEnabled (Variables|Collision|GetCapsuleComponent) "NoCollision")
  (Pawn|Components|CharacterMovement|DisableMovement (Variables|Character|GetCharacterMovement))
  (Pawn|UnPossess (Pawn|GetController)))

(fn IsDead?
  (return false))