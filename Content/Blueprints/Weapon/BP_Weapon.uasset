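; Weapon actor that fires BP_Bullet projectiles automatically while firing is active.
; StartFire and EndFire toggle a firing flag.
; Tick accumulates delta time and, while the flag is set, calls Shoot once the fire-rate interval has elapsed, then resets the timer.
; Shoot spawns the bullet at the weapon mesh's muzzle socket transform in world space.
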(event EventBeginPlay)

(event Collision|EventActorBeginOverlap
  (params (OtherActor :type Actor%20Object%20Reference)))

(event EventTick
  (params (DeltaSeconds :type Float%20%28single-precision%29))
  (Variables|Default|SetfireRateDelta (+ DeltaSeconds (Variables|Default|GetfireRateDelta)))
  (if (and (Variables|Default|GetistFiring) (>= (Variables|Default|GetfireRateDelta) (Variables|Default|GetfireRate)))
    (Variables|Default|SetfireRateDelta 0.0)
    (CallFunction|Shoot)))

(fn ConstructionScript)

(fn Shoot
  (Game|SpawnActorfromClass "/Game/Blueprints/Bullet/BP_Bullet.BP_Bullet_C" (Transformation|GetSocketTransform (Variables|Default|GetWaeponMesh) "MuzzleSocket" "RTS_World") "Undefined" "MultiplyWithRoot" 0 0))

(fn StartFire
  (Variables|Default|SetistFiring true))

(fn EndFire
  (Variables|Default|SetistFiring false))